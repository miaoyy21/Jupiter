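; BP_飞行轨迹 is a flight-trail effect actor that displays a Paper2D flipbook sized to the distance of the current flight.
; On BeginPlay it buckets 本次飞行距离 (flight distance) into fixed steps to pick one of the FB_飞行轨迹 flipbooks.
; After a 持续时间 (duration) delay, a single timeline track drives both uniform scale and sprite alpha, then the actor destroys itself.
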(event EventBeginPlay
  (switch int (Math|Float|Ceil (/ (Variables|Default|Get本次飞行距离) 1.8))
    (:Default
      (Variables|Default|Set图像序列 "/Game/素材/飞行轨迹/FB_飞行轨迹_7.FB_飞行轨迹_7"))
    (:1
      (Variables|Default|Set图像序列 "/Game/素材/飞行轨迹/FB_飞行轨迹_0.FB_飞行轨迹_0"))
    (:2
      (Variables|Default|Set图像序列 "/Game/素材/飞行轨迹/FB_飞行轨迹_1.FB_飞行轨迹_1"))
    (:3
      (Variables|Default|Set图像序列 "/Game/素材/飞行轨迹/FB_飞行轨迹_2.FB_飞行轨迹_2"))
    (:4
      (Variables|Default|Set图像序列 "/Game/素材/飞行轨迹/FB_飞行轨迹_3.FB_飞行轨迹_3"))
    (:5
      (Variables|Default|Set图像序列 "/Game/素材/飞行轨迹/FB_飞行轨迹_4.FB_飞行轨迹_4"))
    (:6
      (Variables|Default|Set图像序列 "/Game/素材/飞行轨迹/FB_飞行轨迹_5.FB_飞行轨迹_5"))
    (:7
      (Variables|Default|Set图像序列 "/Game/素材/飞行轨迹/FB_飞行轨迹_6.FB_飞行轨迹_6")))
  (Sprite|SetFlipbook (Variables|Default|GetPaperFlipbook) (Variables|Default|Get图像序列))
  (Utilities|FlowControl|Delay (Variables|Default|Get持续时间))
  (bind _新建轨道_0 (Timeline|时间轴 Play)
    (:Update
      (Transformation|SetRelativeScale3D (Variables|Default|GetPaperFlipbook) (Math|Vector|MakeVector _新建轨道_0 _新建轨道_0 _新建轨道_0))
      (Sprite|SetSpriteColor (Variables|Default|GetPaperFlipbook) (Utilities|Struct|MakeLinearColor 1.0 1.0 1.0 _新建轨道_0)))
    (:Finished
      (Actor|DestroyActor))))

(fn ConstructionScript)