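; Launch silo turret (发射井) that periodically looks for actors tagged "玩家" (player) within range and fires BP_炮弹 shells at a random one.
; When idle, Tick runs the search, then a timeline pitches it toward the target or back upright.
; A looping timer re-aims and spawns shells for a set duration before searching resumes.
; Outside near-vertical angles, aim adds a fixed lead angle signed by the target's X flight velocity.
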(event Custom|搜索目标
  ;[1 1 1] 搜索可攻击目标
  (Utilities|Array|Clear (Variables|Default|Get可攻击目标列表))
  (bind _outactors (Actor|GetAllActorswithTag "玩家"))
  (for _array_element _outactors
    (if (< (Math|Vector|Distance(Vector) (Transformation|GetActorLocation _array_element) (Transformation|GetActorLocation)) (Math|Float|SelectFloat (Variables|Default|Get搜索最大距离) 1e+05 (> (Variables|Default|Get搜索最大距离) 0.0)))
      (Utilities|Array|Add (Variables|Default|Get可攻击目标列表) _array_element))))

(event Custom|转回初始
  ;[1 1 1] 转向初始方向（垂直90）
  (Variables|Default|Set转向目标初始角度 (Variables|Default|Get转向目标最终角度))
  (Variables|Default|Set转向目标最终角度 9e+01)
  (bind _alpha (Timeline|时间轴_0 PlayFromStart)
    (:Update
      (Transformation|SetActorRotation (Math|Rotator|MakeRotator 0.0 (Math|Float|Lerp (Variables|Default|Get转向目标初始角度) (Variables|Default|Get转向目标最终角度) _alpha) 0.0)))))

(event Custom|攻击目标
  (params (攻击目标 :type Actor%20Object%20Reference))
  ;[1 1 1] 对目标发动攻击
  (bind _returnvalue (Utilities|Time|SetTimerbyEvent (delegate Custom|攻击目标事件) (Variables|Default|Get攻击发动频率) true))
  (Variables|Default|Set攻击目标定时器 _returnvalue)
  (Utilities|FlowControl|Delay (Variables|Default|Get攻击持续时间))
  (Utilities|Time|ClearandInvalidateTimerbyHandle (Variables|Default|Get攻击目标定时器))
  (Variables|Default|Set是否处于攻击中 false))

(event Custom|攻击目标事件
  ;[1 1 1] 对目标发动攻击
  (bind _旋转角度 (CallFunction|FN获得两个位置的旋转角度 (Transformation|GetActorLocation) (Transformation|GetActorLocation (stale Custom|攻击目标 攻击目标))))
  (bind _output_get (Variables|Default|Set转向目标最终角度 _旋转角度))
  (if (or (Math|Float|NearlyEqual(Float) (Math|Float|Absolute(Float) _output_get) 9e+01 3e+01) (Math|Float|NearlyEqual(Float) (Variables|Default|Get攻击预判角度) 0.0 1.0))
    _
    (else
      (bind _飞行速度 (Class|BPI玩家|获取飞行速度3D(Message) (stale Custom|攻击目标 攻击目标)))
      (Variables|Default|Set转向目标最终角度 (+ (* (Math|Float|SelectFloat 1.0 -1.0 (< (.x _飞行速度) 0.0)) (Variables|Default|Get攻击预判角度)) (Variables|Default|Get转向目标最终角度)))))
  (Transformation|SetActorRotation (Math|Rotator|MakeRotator 0.0 (Variables|Default|Get转向目标最终角度) 0.0))
  (Game|SpawnActorfromClass "/Game/蓝图/BP_炮弹.BP_炮弹_C" (Transformation|GetActorTransform) "AdjustIfPossibleButAlwaysSpawn" "MultiplyWithRoot" 0 "/Game/素材/FB_炮弹.FB_炮弹" 2.5e+02 0.0 2.5 0 0.5 0)
  (Variables|Default|Set转向目标初始角度 (Variables|Default|Get转向目标最终角度)))

(event Custom|转向目标
  (params (目标对象 :type Actor%20Object%20Reference))
  ;[1 1 1] 转向目标方向（先转向一次，这样更加自然些）
  (bind _旋转角度 (CallFunction|FN获得两个位置的旋转角度 (Transformation|GetActorLocation) (Transformation|GetActorLocation 目标对象)))
  (Variables|Default|Set转向目标最终角度 _旋转角度)
  (bind _alpha (Timeline|转向目标时间轴 PlayFromStart)
    (:Update
      (Transformation|SetActorRotation (Math|Rotator|MakeRotator 0.0 (Math|Float|Lerp (Variables|Default|Get转向目标初始角度) (Variables|Default|Get转向目标最终角度) _alpha) 0.0)))
    (:Finished
      (Variables|Default|Set转向目标初始角度 (Variables|Default|Get转向目标最终角度))
      (CallFunction|攻击目标 目标对象))))

(event EventBeginPlay
  ;[1 1 1] 开始运行事件
  (Variables|Default|Set转向目标初始角度 (.pitch (Transformation|GetActorRotation self))))

(event EventTick
  (params (DeltaSeconds :type Float%20%28single-precision%29))
  (bind _可攻击目标列表 (Variables|Default|Get可攻击目标列表))
  (bind _outitem (Utilities|Array|Random _可攻击目标列表))
  ;[1 1 1] 每隔一段时间执行搜索可攻击目标
  (if (not (Variables|Default|Get是否处于攻击中))
    (bind _output_get (Variables|Default|Set距离前次搜索执行间隔 (+ DeltaSeconds (Variables|Default|Get距离前次搜索执行间隔))))
    (if (> _output_get (Variables|Default|Get搜索执行间隔))
      (CallFunction|搜索目标)
      (Variables|Default|Set距离前次搜索执行间隔 0.0)
      (Utilities|IsValid _outitem
        (:Is%20Valid
          (Variables|Default|Set是否处于攻击中 true)
          (CallFunction|转向目标 _outitem))
        (:Is%20Not%20Valid
          (Variables|Default|Set是否处于攻击中 false)
          (CallFunction|转回初始))))))

(fn ConstructionScript)

(fn 旋转变换
  (params (旋转 :type Rotator))
  (bind (_roll _pitch _yaw) (Math|Rotator|BreakRotator 旋转))
  (bind _output_get (LocalVariables|SetX _roll))
  (bind _output_get_2 (LocalVariables|SetY _pitch))
  (bind _output_get_3 (LocalVariables|SetZ _yaw))
  (Development|PrintString (Utilities|String|Append (Utilities|String|ToString(Float) _output_get) "," (Utilities|String|ToString(Float) _output_get_2) "," (Utilities|String|ToString(Float) _output_get_3)) true true "(R=0.061271,G=0.186660,B=1.000000,A=1.000000)" 2e+01)
  (if (and (Math|Float|NearlyEqual(Float) (LocalVariables|GetX) 1.8e+02 1.0) (Math|Float|NearlyEqual(Float) (LocalVariables|GetZ) 1.8e+02 1.0))
    (Development|PrintString (Utilities|String|Append " ====>>>> " "0," (Utilities|String|ToString(Float) (- 1.8e+02 (LocalVariables|GetY))) ",0") true true "(R=0.272828,G=0.028347,B=0.380208,A=1.000000)" 2e+01)
    (return (Math|Rotator|MakeRotator 0.0 (- 1.8e+02 (LocalVariables|GetY)) 0.0))
    (elif (and (Math|Float|NearlyEqual(Float) (LocalVariables|GetX) 0.0 1.0) (Math|Float|NearlyEqual(Float) (LocalVariables|GetZ) 1.8e+02 1.0))
      (Development|PrintString (Utilities|String|Append " ====>>>> " "0," (Utilities|String|ToString(Float) (- 1.8e+02 (LocalVariables|GetY))) ",0") true true "(R=0.194603,G=1.000000,B=0.190544,A=1.000000)" 2e+01)
      (return (Math|Rotator|MakeRotator 0.0 (- 1.8e+02 (LocalVariables|GetY)) 0.0))
      (else
        (Development|PrintString (Utilities|String|Append " ====>>>> " "0," (Utilities|String|ToString(Float) (LocalVariables|GetY)) ",0") true true "(R=1.000000,G=0.133849,B=0.183615,A=1.000000)" 2e+01)
        (return (Math|Rotator|MakeRotator 0.0 (LocalVariables|GetY) 0.0))))))