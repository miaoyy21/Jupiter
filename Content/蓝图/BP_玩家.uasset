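; Player character Blueprint that flies at a set speed by writing CharacterMovement velocity directly.
; On BeginPlay it spawns BP_摄像机 as the view target, tags itself 玩家 and starts moving along X; Tick snaps the camera to its location.
; Speed and angle setters rebuild velocity as a pitch-rotated X vector, but 设置旋转角度 always stores zero.
; Getters expose the scalar speed and 3D velocity.
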(event EventBeginPlay
  (bind _returnvalue (Game|SpawnActorfromClass "/Game/蓝图/BP_摄像机.BP_摄像机_C" (Math|Transform|MakeTransform (Transformation|GetActorLocation) "0, 0, 0" "1.000000,1.000000,1.000000") "AdjustIfPossibleButAlwaysSpawn" "MultiplyWithRoot" 0 0))
  (bind _output_get (Variables|Default|Set摄像机 _returnvalue))
  (Game|Player|SetViewTargetwithBlend (Game|GetPlayerController 0) _output_get 0.0 "VTBlend_Linear" 0.0 true)
  (Variables|Default|SetTags (Utilities|Array|MakeArray "玩家"))
  (Variables|/Script/Engine.MovementComponent|SetVelocity (Variables|Character|GetCharacterMovement) (Math|Vector|MakeVector (Variables|Default|Get飞行速度) 0.0 0.0)))

(event EventTick
  (params (DeltaSeconds :type Float%20%28single-precision%29))
  (Transformation|SetActorLocation (Variables|Default|Get摄像机) (Transformation|GetActorLocation) false false))

(event Event设置飞行速度
  (params (飞行速度 :type Float%20%28double-precision%29))
  (bind _output_get (Variables|Default|Set飞行速度 飞行速度))
  (Variables|/Script/Engine.MovementComponent|SetVelocity (Variables|Character|GetCharacterMovement) (Math|Vector|RotateVector (Math|Vector|MakeVector _output_get 0.0 0.0) (Math|Rotator|MakeRotator 0.0 (Variables|Default|Get旋转角度) 0.0))))

(event Event设置旋转角度
  (params (旋转角度 :type Float%20%28double-precision%29))
  (Variables|Default|Set旋转角度 0.0)
  (Variables|/Script/Engine.MovementComponent|SetVelocity (Variables|Character|GetCharacterMovement) (Math|Vector|RotateVector (Math|Vector|MakeVector (Variables|Default|Get飞行速度) 0.0 0.0) (Math|Rotator|MakeRotator 0.0 旋转角度 0.0))))

(fn ConstructionScript
  (|CallParentFunction))

(fn 获取飞行速度
  (return (Variables|Default|Get飞行速度)))

(fn 获取飞行速度3D
  (return (Variables|/Script/Engine.MovementComponent|GetVelocity (Variables|Character|GetCharacterMovement))))