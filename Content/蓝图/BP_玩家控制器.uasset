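; Player controller that drives the BP_玩家 pawn with Enhanced Input for movement on the X and Z axes.
; On BeginPlay it caches the pawn and adds the IMC_映射情境 mapping context.
; The horizontal and vertical actions write a scaled value straight to CharacterMovement velocity instead of adding movement input.
; Each write zeroes the other axes, so the two directions do not combine, and releasing either action stops the pawn.
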(event Input|EnhancedActionEvents|EnhancedInputActionIA_水平移动
  (params (ActionValue :type Float%20%28double-precision%29) (ElapsedSeconds :type Float%20%28double-precision%29) (TriggeredSeconds :type Float%20%28double-precision%29) (InputAction :type Input%20Action%20Object%20Reference :default "/Game/输入/IA_水平移动.IA_水平移动"))
  (bind _玩家 (Variables|Default|Get玩家))
  (bind _charactermovement (Variables|/Script/Engine.Character|GetCharacterMovement _玩家))
  (:Triggered
    (Variables|/Script/Engine.MovementComponent|SetVelocity _charactermovement (Math|Vector|MakeVector (* ActionValue 1e+02) 0.0 0.0)))
  (:Completed
    (Variables|/Script/Engine.MovementComponent|SetVelocity _charactermovement "0, 0, 0")))

(event Input|EnhancedActionEvents|EnhancedInputActionIA_垂直移动
  (params (ActionValue :type Float%20%28double-precision%29) (ElapsedSeconds :type Float%20%28double-precision%29) (TriggeredSeconds :type Float%20%28double-precision%29) (InputAction :type Input%20Action%20Object%20Reference :default "/Game/输入/IA_垂直移动.IA_垂直移动"))
  (bind _玩家 (Variables|Default|Get玩家))
  (bind _charactermovement (Variables|/Script/Engine.Character|GetCharacterMovement _玩家))
  (:Triggered
    (Variables|/Script/Engine.MovementComponent|SetVelocity _charactermovement (Math|Vector|MakeVector 0.0 0.0 (* ActionValue 1e+02))))
  (:Completed
    (Variables|/Script/Engine.MovementComponent|SetVelocity _charactermovement "0, 0, 0")))

(event EventBeginPlay
  (bind _self self)
  (bind _returnvalue (PlayerController|LocalPlayerSubsystems|GetEnhancedInputLocalPlayerSubsystem _self))
  ;[1 1 1] 开始运行事件
  (bind _asbp_玩家 (Utilities|Casting|CastToBP_玩家 (Game|Player|GetPlayerPawn 0)))
  (Variables|Default|Set玩家 _asbp_玩家)
  (Utilities|IsValid _returnvalue
    (:Is%20Valid
      (Input|AddMappingContext _returnvalue "/Game/输入/IMC_映射情境.IMC_映射情境" 0 "(bIgnoreAllPressedKeysUntilRelease=True,bForceImmediately=False,bNotifyUserSettings=False)"))))

(fn ConstructionScript)