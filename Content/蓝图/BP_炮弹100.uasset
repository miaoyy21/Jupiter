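; BP_炮弹100 is a cannonball projectile built with CharacterMovement and a capsule component.
; On BeginPlay it adds one forward-and-up movement input, then sets the movement velocity to a fixed world-space launch vector along +X with some lift.
; An unconnected branch would derive a slower velocity from the capsule's rotation and print it, but it never runs.
; The construction script only calls its parent.
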(event EventBeginPlay
  (Pawn|Input|AddMovementInput "1.000000,0.000000,1.000000" 1.0 false)
  (Variables|/Script/Engine.MovementComponent|SetVelocity (Variables|Character|GetCharacterMovement) "1000.000000,0.000000,200.000000"))

(fn ConstructionScript
  (|CallParentFunction))