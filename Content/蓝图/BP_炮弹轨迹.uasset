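; BP_炮弹轨迹 is a short-lived Paper2D flipbook effect that displays a shell trajectory trail.
; On BeginPlay it assigns the trail flipbook and waits for a configurable duration.
; A timeline then drives both the sprite's Z scale and alpha from a single track, and the actor destroys itself when the timeline finishes.
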(event EventBeginPlay
  (Sprite|SetFlipbook (Variables|Default|GetPaperFlipbook) (Variables|Default|Get炮弹轨迹图像序列))
  (Utilities|FlowControl|Delay (Variables|Default|Get炮弹轨迹持续时间))
  (bind _新建轨道_0 (Timeline|时间轴 Play)
    (:Update
      (Transformation|SetRelativeScale3D (Variables|Default|GetPaperFlipbook) (Math|Vector|MakeVector 1.0 1.0 _新建轨道_0))
      (Sprite|SetSpriteColor (Variables|Default|GetPaperFlipbook) (Utilities|Struct|MakeLinearColor 1.0 1.0 1.0 _新建轨道_0)))
    (:Finished
      (Actor|DestroyActor))))

(fn ConstructionScript)