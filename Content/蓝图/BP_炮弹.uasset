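; BP_炮弹 is a cannon shell projectile drawn with a Paper2D flipbook.
; BeginPlay sets its flipbook and gravity scale, then launches ProjectileMovement along the actor's rotation at the configured initial velocity.
; Each Tick destroys the shell once its flight time limit passes, otherwise spawns a BP_飞行轨迹 trail actor if a trail flipbook is valid.
; A timeline that would rotate the shell and its velocity is left unconnected.
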(event EventBeginPlay
  (bind _returnvalue (Transformation|GetActorRotation))
  (Sprite|SetFlipbook (Variables|Default|GetPaperFlipbook) (Variables|Default|Get【炮弹】图像序列))
  (Variables|Default|Set前帧位置 (Transformation|GetWorldLocation (Variables|Default|GetPaperFlipbook)))
  (Variables|/Script/Engine.ProjectileMovementComponent|SetProjectileGravityScale (Variables|Default|GetProjectileMovement) (Variables|Default|Get【炮弹】重力范围))
  (Variables|Default|Set初始Y轴旋转 (.Pitch (Math|Rotator|BreakRotator _returnvalue)))
  (Variables|/Script/Engine.MovementComponent|SetVelocity (Variables|Default|GetProjectileMovement) (Math|Vector|RotateVector (Math|Vector|MakeVector (Variables|Default|Get【炮弹】初速度) 0.0 0.0) _returnvalue)))

(event EventTick
  (params (DeltaSeconds :type Float%20%28single-precision%29))
  (bind _output_get (Variables|Default|Set当前已飞行时间 (+ DeltaSeconds (Variables|Default|Get当前已飞行时间))))
  (if (> _output_get (Variables|Default|Get【炮弹】飞行时间上限))
    (Actor|DestroyActor)
    (else
      (Utilities|IsValid (Variables|Default|Get【炮弹轨迹】图像序列)
        (:Is%20Valid
          (Game|SpawnActorfromClass "/Game/蓝图/BP_飞行轨迹.BP_飞行轨迹_C" (Transformation|GetActorTransform) "Undefined" "MultiplyWithRoot" 0 (Variables|Default|Get【炮弹轨迹】图像序列) (Variables|Default|Get【炮弹轨迹】持续时间) 0))
        (:Is%20Not%20Valid
          _))
      (Variables|Default|Set当前位置 (Transformation|GetWorldLocation (Variables|Default|GetPaperFlipbook)))
      (Variables|Default|Set前帧位置 (Variables|Default|Get当前位置)))))

(fn ConstructionScript)